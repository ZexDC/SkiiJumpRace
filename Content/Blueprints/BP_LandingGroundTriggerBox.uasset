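; BP_LandingGroundTriggerBox is a landing-zone trigger that measures the player car's jump distance once the race is complete.
; On overlap it disables its overlap events, shows the HUD distance screen and plays its reveal animation.
; If the first BP_JumpCheckpoint reports a valid jump, it stores the horizontal distance from that checkpoint, scaled to meters, on the player controller and saves any new best.
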(event OnComponentBeginOverlap(Box)
  (params (OtherActor :type Actor%20Object%20Reference) (OtherComp :type Primitive%20Component%20Object%20Reference) (OtherBodyIndex :type Integer) (bFromSweep :type Boolean) (SweepResult :type Hit%20Result%20Structure%20%28by%20ref%29))
  (bind _asmy_car (Utilities|Casting|CastToMyCar OtherActor))
  (bind _asmy_player_controller (Utilities|Casting|CastToMyPlayerController (Game|GetPlayerController 0)))
  (bind _output_get (Variables|Default|SetControllerReference _asmy_player_controller))
  (if (Variables|/Game/Blueprints/MyPlayerController.MyPlayerController_C|GetRaceComplete (Variables|Default|GetControllerReference))
    (Variables|/Script/Engine.PrimitiveComponent|SetbGenerateOverlapEvents (Variables|Default|GetBox) false)
    (Variables|/Game/Blueprints/UI/HUD.HUD_C|SetDistanceScreenVisible (Variables|/Game/Blueprints/MyPlayerController.MyPlayerController_C|GetHUDReference _output_get) "Visible")
    (bind _outactors (Actor|GetAllActorsOfClass "/Game/Blueprints/BP_JumpCheckpoint.BP_JumpCheckpoint_C"))
    (Utilities|FlowControl|Sequence
      (:then_0
        (if (Variables|/Game/Blueprints/BP_JumpCheckpoint.BP_JumpCheckpoint_C|GetIsValidJump (Utilities|Array|Get(acopy) _outactors))
          (bind _output_get_2 (Variables|/Game/Blueprints/MyPlayerController.MyPlayerController_C|SetActualDistanceValue (Variables|Default|GetControllerReference) (/ (Transformation|GetHorizontalDistanceTo _asmy_car (Utilities|Array|Get(acopy) _outactors)) 1e+02)))
          (Variables|/Game/Blueprints/MyPlayerController.MyPlayerController_C|SetCurrentDistanceText (Variables|Default|GetControllerReference) (Utilities|Text|ToText(Float) _output_get_2 "HalfToEven" true 1 324 0 2))
          (if (> _output_get_2 (Variables|/Game/Blueprints/MyPlayerController.MyPlayerController_C|GetBestDistanceValue (Variables|Default|GetControllerReference)))
            (bind _output_get_3 (Variables|/Game/Blueprints/MyPlayerController.MyPlayerController_C|SetBestDistanceValue (Variables|Default|GetControllerReference) (Variables|/Game/Blueprints/MyPlayerController.MyPlayerController_C|GetActualDistanceValue (Variables|Default|GetControllerReference))))
            (Variables|/Game/Blueprints/MyPlayerController.MyPlayerController_C|SetBestDistanceText (Variables|Default|GetControllerReference) (Utilities|Text|ToText(Float) _output_get_3 "HalfToEven" true 1 324 0 2))
            (Default|SaveGame (Variables|Default|GetControllerReference)))))
      (:then_1
        (UserInterface|Animation|PlayAnimation (Variables|/Game/Blueprints/MyPlayerController.MyPlayerController_C|GetHUDReference _output_get) (Variables|/Game/Blueprints/UI/HUD.HUD_C|GetShowDistance (Variables|/Game/Blueprints/MyPlayerController.MyPlayerController_C|GetHUDReference _output_get)) 0.0 1 "Forward")))))

(fn ConstructionScript)