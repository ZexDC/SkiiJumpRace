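; Track checkpoint Blueprint that registers when a car drives through it in the intended direction.
; On trigger overlap by MyCar, it dots the car's velocity with the DirectionArrow's forward vector to reject wrong-way crossings.
; A valid pass calls the CheckpointCleared dispatcher with its checkpoint number, then hides the trigger and disables its overlap events so it fires only once.
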(event OnComponentBeginOverlap(Trigger)
  (params (OtherActor :type Actor%20Object%20Reference) (OtherComp :type Primitive%20Component%20Object%20Reference) (OtherBodyIndex :type Integer) (bFromSweep :type Boolean) (SweepResult :type Hit%20Result%20Structure%20%28by%20ref%29))
  ;[1 1 1] Checkpoint system, cleared when overlapping ends
  (bind _asmy_car (Utilities|Casting|CastToMyCar OtherActor))
  (if (> (Math|Vector|DotProduct (Transformation|GetVelocity _asmy_car) (Math|Rotator|GetRotationXVector (Transformation|GetWorldRotation (Variables|Default|GetDirectionArrow)))) 0.0)
    (Default|CallCheckpointCleared (Variables|Default|GetCheckpointNumber))
    (Development|SetHiddeninGame (Variables|Default|GetTrigger) true false)
    (Variables|/Script/Engine.PrimitiveComponent|SetbGenerateOverlapEvents (Variables|Default|GetTrigger) false)))

(fn ConstructionScript)