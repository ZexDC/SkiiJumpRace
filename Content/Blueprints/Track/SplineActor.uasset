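; Spline-driven track actor that builds a floor surface along its Spline.
; The construction script adds a collidable Floor_400x400 spline mesh at each Spacing interval along the spline's length.
; Each segment takes its ends from local-space spline positions and its tangents from the spline direction multiplied by TangentScale.
; Actor overlap only prints a message that a new spline point is needed; no points are added at runtime.
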(event EventBeginPlay)

(event EventActorBeginOverlap
  (params (OtherActor :type Actor%20Object%20Reference))
  (Development|PrintString "Trigger activated, need new spline point"))

(event EventTick
  (params (DeltaSeconds :type Float%20%28single-precision%29)))

(fn ConstructionScript
  (bind _spline (Variables|Default|GetSpline))
  (bind _tangentscale (Variables|Default|GettangentScale))
  (bind _spacing (Variables|Default|GetSpacing))
  (for _index (range 0 (Math|Float|Truncate (/ (Spline|GetSplineLength (Variables|Default|GetSpline)) (Variables|Default|GetSpacing))))
    (bind _returnvalue (AddComponent|AddSplineMeshComponent false))
    (Collision|SetCollisionEnabled _returnvalue "QueryAndPhysics")
    (Components|StaticMesh|SetStaticMesh _returnvalue "/Game/StarterContent/Architecture/Floor_400x400.Floor_400x400")
    (Rendering|Material|SetMaterial _returnvalue 0 "/Game/Materials/02_-_Default.02_-_Default")
    (SplineMesh|SetStartandEnd _returnvalue (Spline|GetLocationatDistanceAlongSpline _spline (* _index _spacing) "Local") (* (Spline|GetDirectionatDistanceAlongSpline _spline (* _index _spacing) "Local") _tangentscale) (Spline|GetLocationatDistanceAlongSpline _spline (+ (* _index _spacing) _spacing) "Local") (* (Spline|GetDirectionatDistanceAlongSpline _spline (+ (* _index _spacing) _spacing) "Local") _tangentscale) :!class /Script/Engine.SplineMeshComponent)))