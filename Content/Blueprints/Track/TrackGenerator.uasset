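; Spline-driven track generator that builds a road with optional left and right guardrails in its construction script.
; It resizes a per-point road data array to match the spline points, then adds spline mesh components per segment, interpolating bank, width and thickness between neighboring points.
; A looping flag closes the circuit.
; Optional text renders number the track points, and a collision toggle avoids editor lag.
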(fn ConstructionScript
  (bind _roaddataarray (Variables|TrackSetup|GetRoadDataArray))
  (Utilities|FlowControl|Sequence
    (:then_0
      ;[1 1 1] Store number of spline points
      (Variables|Default|SetSplinePointsNumber (Spline|GetNumberOfSplinePoints (Variables|Default|GetSpline))))
    (:then_1
      ;[1 1 1] Check that road data array has same number of spline points
      (Math|Integer|CompareInt (Utilities|Array|Length (Variables|TrackSetup|GetRoadDataArray)) (Variables|Default|GetSplinePointsNumber) :!label _label
        (:>
          (Utilities|Array|RemoveIndex _roaddataarray (Utilities|Array|LastIndex _roaddataarray))
          (goto _label))
        (:<
          (Utilities|Array|Add (Variables|TrackSetup|GetRoadDataArray) (Variables|Default|GetRoadMeshDefaults))
          (goto _label))))
    (:then_2
      ;[1 1 1] Build track mesh for each spline segment
      (for _index (range 0 (- (Variables|Default|GetSplinePointsNumber) (Math|Integer|SelectInt 1 2 (Variables|TrackSetup|GetLoopingTrack))))
        (Variables|Default|SetCurrentLoopIndex _index)
        ;;[1 1 1] Store left/right guardrail data
        (Variables|Default|SetDrawLeftGuardRail (.leftguardrail (Utilities|Array|Get(acopy) (Variables|TrackSetup|GetRoadDataArray) (Variables|Default|GetCurrentLoopIndex))))
        (Variables|Default|SetDrawRightGuardRail (.rightguardrail (Utilities|Array|Get(acopy) (Variables|TrackSetup|GetRoadDataArray) (Variables|Default|GetCurrentLoopIndex))))
        (Utilities|FlowControl|Sequence
          (:then_0
            (CallFunction|BuildTrackElement (Variables|Default|GetCurrentLoopIndex) (Variables|TrackMeshes|GetRoadMesh)))
          (:then_1
            (if (Variables|Default|GetDrawLeftGuardRail)
              (CallFunction|BuildTrackElement (Variables|Default|GetCurrentLoopIndex) (Variables|TrackMeshes|GetLeftGuardRailMesh))))
          (:then_2
            (if (Variables|Default|GetDrawRightGuardRail)
              (CallFunction|BuildTrackElement (Variables|Default|GetCurrentLoopIndex) (Variables|TrackMeshes|GetRightGuardRailMesh)))))))
    (:then_3
      ;[1 1 1] Draw track point numbers if enabled
      (if (Variables|TrackDebug|GetDrawTrackPointNumbers)
        (for _index_2 (range 0 (- (Variables|Default|GetSplinePointsNumber) (Math|Integer|SelectInt 1 2 (Variables|TrackSetup|GetLoopingTrack))))
          (Variables|Default|SetCurrentTrackPoint (Utilities|Text|ToText(Integer) _index_2))
          (bind _returnvalue (AddComponent|AddTextRenderComponent false (Math|Transform|MakeTransform (Math|Vector|MakeVector (.X (Math|Vector|BreakVector (.Location (Spline|GetLocationandTangentatSplinePoint (Variables|Default|GetSpline) _index_2 "Local")))) (.Y (Math|Vector|BreakVector (.Location (Spline|GetLocationandTangentatSplinePoint (Variables|Default|GetSpline) _index_2 "Local")))) (+ (.Z (Math|Vector|BreakVector (.Location (Spline|GetLocationandTangentatSplinePoint (Variables|Default|GetSpline) _index_2 "Local")))) 5e+01)) (Math|Conversions|RotationFromXVector (* (.Tangent (Spline|GetLocationandTangentatSplinePoint (Variables|Default|GetSpline) _index_2 "Local")) -1)))))
          (Rendering|Components|TextRender|SetText _returnvalue (Variables|Default|GetCurrentTrackPoint)))))))

(fn BuildTrackElement
  (params (LoopIndex :type Integer) (TrackElementMesh :type Static%20Mesh%20Object%20Reference))
  (LocalVariables|SetLocal_CurrentLoopIndex LoopIndex)
  (LocalVariables|SetLocal_NextLoopIndex (Math|Integer|%(Integer) (+ LoopIndex 1) (Variables|Default|GetSplinePointsNumber)))
  (LocalVariables|SetLocal_TrackElementMesh TrackElementMesh)
  (Utilities|FlowControl|Sequence
    (:then_0
      ;[1 1 1] Store relevant data for each track element
      (LocalVariables|SetLocal_StartLocation (.Location (Spline|GetLocationandTangentatSplinePoint (Variables|Default|GetSpline) (LocalVariables|GetLocal_CurrentLoopIndex) "Local")))
      (LocalVariables|SetLocal_StartTangent (.Tangent (Spline|GetLocationandTangentatSplinePoint (Variables|Default|GetSpline) (LocalVariables|GetLocal_CurrentLoopIndex) "Local")))
      (LocalVariables|SetLocal_EndLocation (.Location (Spline|GetLocationandTangentatSplinePoint (Variables|Default|GetSpline) (LocalVariables|GetLocal_NextLoopIndex) "Local")))
      (LocalVariables|SetLocal_EndTangent (.Tangent (Spline|GetLocationandTangentatSplinePoint (Variables|Default|GetSpline) (LocalVariables|GetLocal_NextLoopIndex) "Local")))
      (LocalVariables|SetLocal_StartRoll (.trackbank (Utilities|Array|Get(acopy) (Variables|TrackSetup|GetRoadDataArray) (LocalVariables|GetLocal_CurrentLoopIndex))))
      (LocalVariables|SetLocal_StartScale (Math|Vector2D|MakeVector2D (.trackwidth (Utilities|Array|Get(acopy) (Variables|TrackSetup|GetRoadDataArray) (LocalVariables|GetLocal_CurrentLoopIndex))) (.trackthickness (Utilities|Array|Get(acopy) (Variables|TrackSetup|GetRoadDataArray) (LocalVariables|GetLocal_CurrentLoopIndex)))))
      (LocalVariables|SetLocal_EndRoll (.trackbank (Utilities|Array|Get(acopy) (Variables|TrackSetup|GetRoadDataArray) (LocalVariables|GetLocal_NextLoopIndex))))
      (LocalVariables|SetLocal_EndScale (Math|Vector2D|MakeVector2D (.trackwidth (Utilities|Array|Get(acopy) (Variables|TrackSetup|GetRoadDataArray) (LocalVariables|GetLocal_NextLoopIndex))) (.trackthickness (Utilities|Array|Get(acopy) (Variables|TrackSetup|GetRoadDataArray) (LocalVariables|GetLocal_NextLoopIndex))))))
    (:then_1
      ;[1 1 1] Use stored data to build track element
      (bind _returnvalue (AddComponent|AddSplineMeshComponent false))
      (LocalVariables|SetLocal_CurrentSplineMesh _returnvalue)
      (Components|StaticMesh|SetStaticMesh (LocalVariables|GetLocal_CurrentSplineMesh) (LocalVariables|GetLocal_TrackElementMesh))
      (SplineMesh|SetStartandEnd (LocalVariables|GetLocal_CurrentSplineMesh) (LocalVariables|GetLocal_StartLocation) (LocalVariables|GetLocal_StartTangent) (LocalVariables|GetLocal_EndLocation) (LocalVariables|GetLocal_EndTangent) :!class /Script/Engine.SplineMeshComponent)
      (Class|SplineMeshComponent|SetStartRoll (LocalVariables|GetLocal_CurrentSplineMesh) (LocalVariables|GetLocal_StartRoll))
      (Class|SplineMeshComponent|SetEndRoll (LocalVariables|GetLocal_CurrentSplineMesh) (LocalVariables|GetLocal_EndRoll))
      (SplineMesh|SetStartScale (LocalVariables|GetLocal_CurrentSplineMesh) (LocalVariables|GetLocal_StartScale) :!class /Script/Engine.SplineMeshComponent)
      (SplineMesh|SetEndScale (LocalVariables|GetLocal_CurrentSplineMesh) (LocalVariables|GetLocal_EndScale) :!class /Script/Engine.SplineMeshComponent)
      ;[1 1 1] Set collision (off while in editor to avoid lag)
      (Collision|SetCollisionEnabled (LocalVariables|GetLocal_CurrentSplineMesh) (select (Variables|TrackDebug|GetCollisions) "QueryAndPhysics" "NoCollision")))))