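; Player-driven race car that passes throttle, steering and handbrake input to its vehicle movement once the race starts.
; Throttle sign and forward speed set brake and reverse lights; speed also drives engine audio.
; It toggles in-car and chase cameras, with pitch-clamped chase orbit.
; When stuck, a delayed recheck shows a respawn prompt; confirming destroys the car and calls the player controller's respawn, while off-track respawn logic is disconnected.
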(event EventTick
  (params (DeltaSeconds :type Float%20%28single-precision%29))
  (bind _controllerreference (Variables|Default|GetControllerReference))
  (bind _controllerreference_2 (Variables|Default|GetControllerReference))
  (bind _controllerreference_3 (Variables|Default|GetControllerReference))
  (bind _hudreference (Variables|/Game/Blueprints/MyPlayerController.MyPlayerController_C|GetHUDReference _controllerreference_2))
  ;[1 1 1] Update
  (if (Variables|/Game/Blueprints/MyPlayerController.MyPlayerController_C|GetRaceStart _controllerreference)
    (Input|EnableInput _controllerreference)
    (Utilities|FlowControl|Sequence
      (:then_0
        ;[1 1 1] Audio
        (Audio|Parameter|SetFloatParameter (Variables|Default|GetEngineSound) "RPM" (Math|Float|Absolute(Float) (Vehicle|GetForwardSpeed (Variables|Default|GetVehicleMovement))) :!class /Script/Engine.AudioComponent))
      (:then_1
        ;[1 1 1] Check if player is stuck, if so, make respawn available and call respawn in MyPlayerController
        (bind _isplayerstuck (CallFunction|StuckCheck))
        (if _isplayerstuck
          (Utilities|FlowControl|Delay 1.65)
          (bind _isplayerstuck_2 (CallFunction|StuckCheck))
          (if _isplayerstuck_2
            (Variables|/Game/Blueprints/UI/HUD.HUD_C|SetRespawnPopupVisible _hudreference "Visible")
            (if (or (Game|Player|IsInputKeyDown _controllerreference_3 "Gamepad_Special_Left") (Game|Player|IsInputKeyDown _controllerreference_3 "R"))
              (Actor|DestroyActor))
            (else
              (Variables|/Game/Blueprints/UI/HUD.HUD_C|SetRespawnPopupVisible _hudreference "Hidden" :!label _label)))
          (else
            (goto _label)))))))

(event EventDestroyed
  (Default|RespawnVehicle (Variables|Default|GetControllerReference)))

(event EventBeginPlay
  ;[1 1 1] Game Start, get reference and set respawn
  (bind _asmy_player_controller (Utilities|Casting|CastToMyPlayerController (Game|GetPlayerController 0)))
  (bind _output_get (Variables|Default|SetControllerReference _asmy_player_controller))
  (Variables|/Game/Blueprints/MyPlayerController.MyPlayerController_C|SetRespawnLocation _output_get (Transformation|GetActorTransform))
  (Input|DisableInput (Variables|Default|GetControllerReference))
  (Camera|EnableinCarView true))

(event Input|ActionEvents|InputActionSwitchCamera
  (params (Key :type Key%20Structure :default "AnyKey"))
  ;[1 1 1] Handle Camera switching
  (:Pressed
    (Camera|EnableinCarView (not (Variables|Camera|GetIsInCar)))))

(event Input|ActionEvents|InputActionHandbrake
  (params (Key :type Key%20Structure :default "AnyKey"))
  (bind _vehiclemovement (Variables|Default|GetVehicleMovement))
  ;[1 1 1] Handbrake Input
  (:Pressed
    (Class|WheeledVehicleMovementComponent|SetHandbrakeInput _vehiclemovement true))
  (:Released
    (Class|WheeledVehicleMovementComponent|SetHandbrakeInput _vehiclemovement false)))

(event Input|AxisEvents|InputAxisCameraPitch
  (params (AxisValue :type Float%20%28single-precision%29))
  (bind _springarm (Variables|Camera|GetSpringArm))
  (bind _returnvalue (Transformation|GetWorldRotation _springarm))
  (bind (_roll _pitch _yaw) (Math|Rotator|BreakRotator _returnvalue))
  ;[1 1 1] Control ChaseCamera Axis Pitch (Up/Down) if not in-car view
  (if (not (Variables|Camera|GetIsInCar))
    ;;[1 1 1] Limit pitch between -70 and 15 to avoid bad camera positioning/stuttering
    (Variables|Default|SetPitch (+ _pitch (* AxisValue (Variables|Default|GetCameraAxisRate) (Utilities|Time|GetWorldDeltaSeconds))))
    (if (> (Variables|Default|GetPitch) 15.0)
      (Variables|Default|SetPitch 15.0)
      (elif (< (Variables|Default|GetPitch) -7e+01)
        (Variables|Default|SetPitch -7e+01)))
    (Transformation|SetWorldRotation (Variables|Camera|GetSpringArm) (Math|Rotator|MakeRotator 0.0 (Variables|Default|GetPitch) _yaw) false false)))

(event Input|AxisEvents|InputAxisForward
  (params (AxisValue :type Float%20%28single-precision%29))
  ;[1 1 1] Accelerate/Decelerate Input
  (Class|WheeledVehicleMovementComponent|SetThrottleInput (Variables|Default|GetVehicleMovement) AxisValue)
  (CarEffects|HandleCarLights AxisValue))

(event Input|AxisEvents|InputAxisRight
  (params (AxisValue :type Float%20%28single-precision%29))
  ;[1 1 1] Steering Input
  (Class|WheeledVehicleMovementComponent|SetSteeringInput (Variables|Default|GetVehicleMovement) AxisValue))

(event Input|AxisEvents|InputAxisCameraYaw
  (params (AxisValue :type Float%20%28single-precision%29))
  (bind _springarm (Variables|Camera|GetSpringArm))
  (bind _returnvalue (Transformation|GetWorldRotation _springarm))
  (bind (_roll _pitch _yaw) (Math|Rotator|BreakRotator _returnvalue))
  ;[1 1 1] Control ChaseCamera Axis Yaw (Left/Right) if not in-car view
  (if (not (Variables|Camera|GetIsInCar))
    (Transformation|SetWorldRotation _springarm (Math|Rotator|MakeRotator 0.0 _pitch (+ _yaw (* AxisValue (Variables|Default|GetCameraAxisRate) (Utilities|Time|GetWorldDeltaSeconds)))) false false)))

(fn ConstructionScript)

(fn EnableinCarView
  (params (State :type Boolean))
  (bind _internalcamera (Variables|Camera|GetInternalCamera))
  (bind _chasecamera (Variables|Camera|GetChaseCamera))
  (bind _output_get (Variables|Camera|SetIsInCar State))
  (if _output_get
    ;[1 1 1] Activate Internal, Deactivate chase
    (Components|Activation|Activate _internalcamera false)
    (Components|Activation|Deactivate _chasecamera)
    (else
      ;[1 1 1] Deactivate Internal, Activate chase
      (Components|Activation|Deactivate _internalcamera)
      (Components|Activation|Activate _chasecamera false))))

(fn StuckCheck
  ;[1 1 1] Check to see if player is not moving
  (if (Variables|/Game/Blueprints/MyPlayerController.MyPlayerController_C|GetRaceComplete (Variables|Default|GetControllerReference)) ; If the race is complete do not check if it is stuck, but set it as not stuck
    (Variables|Default|SetIsStuck false :!label _label)
    (elif (< (Vehicle|GetForwardSpeed (Variables|Default|GetVehicleMovement)) 2.5)
      (Variables|Default|SetIsStuck true)
      (else
        (goto _label))))
  (return (Variables|Default|GetIsStuck)))

(fn EnableBrakeLights
  ;[1 1 1] Left light intensity
  (Rendering|Components|Light|SetIntensity (Variables|Default|GetBrakeLightLeft) 2.4e+03)
  ;[1 1 1] Right light intensity
  (Rendering|Components|Light|SetIntensity (Variables|Default|GetBrakeLightRight) 2.4e+03))

(fn DisableBrakeLights
  ;[1 1 1] Left light intensity
  (Rendering|Components|Light|SetIntensity (Variables|Default|GetBrakeLightLeft) 4e+02)
  ;[1 1 1] Right light intensity
  (Rendering|Components|Light|SetIntensity (Variables|Default|GetBrakeLightRight) 4e+02))

(fn ReverseCheck
  (if (< (.x (Transformation|GetVelocity)) 0.0)
    (return true)
    (else
      (return false))))

(fn HandleCarLights
  (params (AxisThrottleValue :type Float%20%28single-precision%29))
  (if (< AxisThrottleValue 0.0)
    (if (< (Vehicle|GetForwardSpeed (Variables|Default|GetVehicleMovement)) 0.0)
      ;[1 1 1] Reversing
      (CarEffects|DisableBrakeLights)
      (CarEffects|EnableReverseLights)
      (else
        ;[1 1 1] Breaking
        (CarEffects|DisableReverseLights)
        (CarEffects|EnableBrakeLights)))
    (else
      ;[1 1 1] Not breaking/reversing
      (CarEffects|DisableBrakeLights)
      (CarEffects|DisableReverseLights))))

(fn EnableReverseLights
  ;[1 1 1] Left light intensity
  (Rendering|Components|Light|SetIntensity (Variables|Default|GetReverseLightLeft) 8e+02)
  ;[1 1 1] Right light intensity
  (Rendering|Components|Light|SetIntensity (Variables|Default|GetReverseLightRight) 8e+02))

(fn DisableReverseLights
  ;[1 1 1] Left light intensity
  (Rendering|Components|Light|SetIntensity (Variables|Default|GetReverseLightLeft) 0.0)
  ;[1 1 1] Right light intensity
  (Rendering|Components|Light|SetIntensity (Variables|Default|GetReverseLightRight) 0.0))

(fn GetJumpMeasure
  (bind _jumpcheckpointreference (LocalVariables|GetJumpCheckpointReference))
  (if (Variables|/Game/Blueprints/BP_JumpCheckpoint.BP_JumpCheckpoint_C|GetIsValidJump _jumpcheckpointreference)
    (return (Transformation|GetHorizontalDistanceTo _jumpcheckpointreference))
    (else
      (return 0.0))))

(fn OffTrackCheck
  (if (Game|Player|IsInputKeyDown (Variables|Default|GetControllerReference) "T")
    (Variables|Default|SetIsOffTrack true)
    (else
      (Variables|Default|SetIsOffTrack false)))
  (return (Variables|Default|GetIsOffTrack)))