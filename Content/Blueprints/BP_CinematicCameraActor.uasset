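; BP_CinematicCameraActor is a cinematic camera actor that follows the car during a valid jump.
; Each tick it reads IsValidJump from the first BP_JumpCheckpoint found and, when true, turns to face the first MyCar.
; Beyond a maximum distance, it steps forward along its local X axis to close in on the car.
; Orbit logic around the car is present but disconnected.
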(event EventTick
  (params (DeltaSeconds :type Float%20%28single-precision%29))
  ;[1 1 1] Point cinematic camera to car
  (bind _outactors (Actor|GetAllActorsOfClass "/Game/Blueprints/BP_JumpCheckpoint.BP_JumpCheckpoint_C"))
  (if (Variables|/Game/Blueprints/BP_JumpCheckpoint.BP_JumpCheckpoint_C|GetIsValidJump (Utilities|Array|Get(acopy) _outactors))
    (bind _outactors_2 (Actor|GetAllActorsOfClass "/Game/Blueprints/Car/MyCar.MyCar_C"))
    (Transformation|SetActorRotation (Math|Rotator|FindLookatRotation (Transformation|GetActorLocation) (Transformation|GetActorLocation (Utilities|Array|Get(acopy) _outactors_2))))
    ;[1 1 1] Move camera towards the car
    (if (> (Transformation|GetDistanceTo (Utilities|Array|Get(acopy) _outactors_2)) 1.3e+03)
      (Transformation|AddActorLocalOffset "50.000000,0.000000,0.000000" false false))))

(fn ConstructionScript)