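; BP_JumpCheckpoint is a checkpoint that validates a car jump and switches the player's view to a cinematic camera.
; When a MyCar leaves the trigger, a dot product of its velocity and the direction arrow's forward vector confirms the correct travel direction.
; A pass sets IsValidJump, then after a short delay cuts the car controller's view to the first BP_CinematicCameraActor found in the level.
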(event OnComponentEndOverlap(Trigger)
  (params (OtherActor :type Actor%20Object%20Reference) (OtherComp :type Primitive%20Component%20Object%20Reference) (OtherBodyIndex :type Integer))
  ;[1 1 1] Validate jump if checkpoint cleared
  (bind _asmy_car (Utilities|Casting|CastToMyCar OtherActor))
  (if (> (Math|Vector|DotProduct (Transformation|GetVelocity _asmy_car) (Math|Rotator|GetRotationXVector (Transformation|GetWorldRotation (Variables|Default|GetDirectionArrow)))) 0.0)
    (Variables|Default|SetIsValidJump true)
    ;[1 1 1] Set view on cinematic camera
    (bind _outactors (Actor|GetAllActorsOfClass "/Game/Blueprints/BP_CinematicCameraActor.BP_CinematicCameraActor_C"))
    (Utilities|FlowControl|Delay 0.5)
    (Game|Player|SetViewTargetwithBlend (Variables|/Game/Blueprints/Car/MyCar.MyCar_C|GetControllerReference _asmy_car) (Utilities|Array|Get(acopy) _outactors) 0.0 "VTBlend_Linear" 0.0 false)))

(fn ConstructionScript)